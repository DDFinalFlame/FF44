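; Stage 02 dungeon room Blueprint that runs the Sevarog introduction cinematic.
; On BeginPlay it binds to the cinematic trigger in its StartTrigger child actor; triggering blends the player view to this actor and plays the CinematicCameraActor sequence.
; Sequencer events show the Sevarog name widget, then blend the view back to the controlled pawn, stop the sequence and remove the widget.
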(event `self.ReceiveBeginPlay`
  (bind _asbp_sevarog_cinematic_trigger (cast `/Enemy/Content/BP_SevarogCinematicTrigger` (`ChildActorComponent.ChildActor` (`self.StartTrigger`))))
  (add `BossCinematicTrigger.OnCinematicTriggered` _asbp_sevarog_cinematic_trigger (delegate `Trigger`)))

(event `Trigger`
  (params (OtherActor :type "Actor Object Reference"))
  (`PlayerController.SetViewTargetWithBlend` (`GameplayStatics.GetPlayerController` 0) self 2.0 "VTBlend_Linear" 0.0 false)
  (`ActorSequenceComponent.PlaySequence` (`self.CinematicCameraActor`)))

(event `SequenceEvent_1`
  (bind _returnvalue (`GameplayStatics.GetPlayerController` 0))
  (`PlayerController.SetViewTargetWithBlend` _returnvalue (`Controller.K2_GetPawn` _returnvalue) 2.0 "VTBlend_Linear" 0.0 false)
  (`ActorSequenceComponent.StopSequence` (`self.CinematicCameraActor`))
  (`Widget.RemoveFromParent` (`self.NameUI`)))

(event `StartNameUI`
  (bind _returnvalue (`|CreateWidget` "/Game/Assets/UI/Boss/WB_SevarogName.WB_SevarogName_C" :!label _label))
  (bind _output_get (set `self.NameUI` _returnvalue))
  (`UserWidget.AddToViewport` _output_get 0))

(event `SequenceEvent`
  (goto _label))

(event `SequenceEvent_0`)

(fn `UserConstructionScript`)