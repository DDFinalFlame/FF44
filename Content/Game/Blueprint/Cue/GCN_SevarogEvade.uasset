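; Looping GameplayCue notify for boss Sevarog's evade, adding shadow-trail particles while the cue is active.
; On looping start it casts the target to BP_BossSevarog, attaches the trail emitter to the mesh root and spawns an attached audio component with no sound specified.
; On removal it deactivates and destroys stored effects, stopping and destroying the audio inside that same loop.
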(event `self.OnLoopingStart`
  (params (Target :type "Actor Object Reference") (Parameters :type "GameplayCueParameters Structure (by ref)") (SpawnResults :type "GameplayCueNotify_SpawnResult Structure (by ref)"))
  (bind _asbp_boss_sevarog (cast `/Game/Game/Blueprint/Monster/Sevarog/BP_BossSevarog` Target))
  (bind _mesh (`Character.Mesh` _asbp_boss_sevarog))
  (bind _returnvalue (`GameplayStatics.SpawnEmitterAttached` "/Game/Assets/SkeletalMesh/Monster/Sevarog/FX/CA/P_ShadowTrails.P_ShadowTrails" _mesh "root" (0.0 0.0 -5.0)))
  (set `self.FX` (`|MakeArray` _returnvalue))
  (bind _returnvalue_2 (`GameplayStatics.SpawnSoundAttached` null _mesh "None" (0.0 0.0 0.0) (struct) "KeepRelativeOffset" false 1.0 1.0 0.0 null null))
  (set `self.AudioComponent` _returnvalue_2))

(event `self.OnRemoval`
  (params (Target :type "Actor Object Reference") (Parameters :type "GameplayCueParameters Structure (by ref)") (SpawnResults :type "GameplayCueNotify_SpawnResult Structure (by ref)"))
  (bind _audiocomponent (`self.AudioComponent`))
  (bind _fx (`self.FX`))
  (for _array_element _fx
    (`ActorComponent.Deactivate` _array_element)
    (`ActorComponent.K2_DestroyComponent` _array_element null)
    (`AudioComponent.Stop` _audiocomponent)
    (`ActorComponent.K2_DestroyComponent` _audiocomponent null))
  (`KismetArrayLibrary.Array_Clear` _fx))

(fn `UserConstructionScript`)