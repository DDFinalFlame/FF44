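; Player gameplay ability for a special hit reaction where the player is grabbed by the attacker.
; On commit it plays hurt sounds and a hit montage, attaches the player to the hand socket of the mesh passed in the event's OptionalObject and disables movement.
; It applies a damage effect built from the instigator's ASC, repeating attach and damage on each notify begin.
; The "Fall" notify end restores walking and ends the ability, which detaches the player.
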(event `self.K2_ActivateAbilityFromEvent`
  (params (EventData :type "GameplayEventData Structure (by ref)"))
  (bind _asbase_player (cast `BasePlayer` (`.AvatarActor` (break `GameplayAbilityActorInfo` (`self.GetActorInfo`)))))
  (set `self.Base Player` _asbase_player)
  (bind _returnvalue (`self.K2_CommitAbility`))
  (if (not _returnvalue)
    (`self.K2_EndAbility`)))

(event `self.K2_CommitExecute`
  (bind _returnvalue (`AbilitySystemBlueprintLibrary.GetAbilitySystemComponent` (`self.Base Player`)))
  (`GameplayStatics.PlaySound2D` "/Game/Assets/SFX/Player/Voice/voice_male_c_hurt_pain_Cue.voice_male_c_hurt_pain_Cue" 1.0 1.0 0.0 null null)
  (`GameplayStatics.PlaySound2D` "/Game/Assets/SFX/Player/Hit/Armor_hit.Armor_hit" 1.0 1.0 0.0 null null)
  (bind _notifyname (`|PlayMontage` (`Character.Mesh` (`self.Base Player`)) (`self.HitMontage`))
    (:`then`
      (`|ExecutionSequence` :!label _label
        (:`then_0`
          (bind `_as스태틱_메시_컴포넌트` (cast `StaticMeshComponent` (`.OptionalObject` (break `GameplayEventData` (stale `self.K2_ActivateAbilityFromEvent` EventData)))))
          (`Actor.K2_AttachToComponent` (`self.Base Player`) `_as스태틱_메시_컴포넌트` "Hand_Middle_Socket" "SnapToTarget" "KeepWorld" "KeepWorld" true)
          (`CharacterMovementComponent.DisableMovement` (`Character.CharacterMovement` (`self.Base Player`))))
        (:`then_1`
          (bind _returnvalue_2 (`AbilitySystemBlueprintLibrary.GetAbilitySystemComponent` (`.Instigator` (break `GameplayEventData` (stale `self.K2_ActivateAbilityFromEvent` EventData)))))
          (`/Engine/EditorBlueprintResources/StandardMacros.IsValid` _returnvalue_2
            (:`Is Valid`
              (`/Engine/EditorBlueprintResources/StandardMacros.IsValid` _returnvalue
                (:`Is Valid`
                  (`AbilitySystemComponent.BP_ApplyGameplayEffectSpecToSelf` _returnvalue (`AbilitySystemComponent.MakeOutgoingSpec` _returnvalue_2 (`self.GE_Damaged`) 0.0 (`.ContextHandle` (break `GameplayEventData` (stale `self.K2_ActivateAbilityFromEvent` EventData))))))))))))
    (:`OnCompleted`
      (`self.K2_EndAbility` :!label _label_2))
    (:`OnBlendOut`
      (goto _label_2))
    (:`OnInterrupted`
      (goto _label_2))
    (:`OnNotifyBegin`
      (goto _label))
    (:`OnNotifyEnd`
      (if (== _notifyname "Fall")
        (`CharacterMovementComponent.SetMovementMode` (`Character.CharacterMovement` (`self.Base Player`)) "MOVE_Walking" 0)
        (goto _label_2)))))

(event `self.K2_OnEndAbility`
  (params (bWasCancelled :type Boolean))
  (`Actor.K2_DetachFromActor` (`self.Base Player`) "KeepWorld" "KeepWorld" "KeepWorld")
  (`parent.K2_OnEndAbility` bWasCancelled))