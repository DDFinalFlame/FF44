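; Gameplay ability for the player's hit reaction, activated by a gameplay event.
; On commit it plays pain and armor-hit sounds and the hit montage, and it ends immediately if the commit fails.
; When the montage blends in, the instigator's ability system builds the GEDamaged effect spec, which the target's applies to itself.
; The ability ends when the montage completes, blends out, is interrupted or is cancelled.
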(event `self.K2_ActivateAbilityFromEvent`
  (params (EventData :type "GameplayEventData Structure (by ref)"))
  (bind _returnvalue (`self.K2_CommitAbility`))
  (if (not _returnvalue)
    (`self.K2_EndAbility`)))

(event `self.K2_CommitExecute`
  (`GameplayStatics.PlaySound2D` "/Game/Assets/SFX/Player/Voice/voice_male_c_hurt_pain_Cue.voice_male_c_hurt_pain_Cue" 1.0 1.0 0.0 null null)
  (`GameplayStatics.PlaySound2D` "/Game/Assets/SFX/Player/Hit/Armor_hit.Armor_hit" 1.0 1.0 0.0 null null)
  (`AbilityTask_PlayMontageAndWait.CreatePlayMontageAndWaitProxy` "None" (`self.HitMontage`)
    (:`OnCompleted`
      (`self.K2_EndAbility` :!label _label))
    (:`OnBlendedIn`
      (bind _returnvalue (`AbilitySystemBlueprintLibrary.GetAbilitySystemComponent` (`.Instigator` (break `GameplayEventData` (stale `self.K2_ActivateAbilityFromEvent` EventData)))))
      (`/Engine/EditorBlueprintResources/StandardMacros.IsValid` _returnvalue
        (:`Is Valid`
          (bind _returnvalue_2 (`AbilitySystemBlueprintLibrary.GetAbilitySystemComponent` (`.Target` (break `GameplayEventData` (stale `self.K2_ActivateAbilityFromEvent` EventData)))))
          (`/Engine/EditorBlueprintResources/StandardMacros.IsValid` _returnvalue_2
            (:`Is Valid`
              (`AbilitySystemComponent.BP_ApplyGameplayEffectSpecToSelf` _returnvalue_2 (`AbilitySystemComponent.MakeOutgoingSpec` _returnvalue (`self.GE_Damaged`) 0.0 (`.ContextHandle` (break `GameplayEventData` (stale `self.K2_ActivateAbilityFromEvent` EventData))))))))))
    (:`OnBlendOut`
      (goto _label))
    (:`OnInterrupted`
      (goto _label))
    (:`OnCancelled`
      (goto _label))))

(event `self.K2_OnEndAbility`
  (params (bWasCancelled :type Boolean)))