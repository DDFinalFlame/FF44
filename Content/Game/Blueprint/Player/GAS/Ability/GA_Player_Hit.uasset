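; GA_Player_Hit is the player's hit-reaction gameplay ability, activated by a gameplay event that carries the hit data.
; Activation stores the event data and commits, ending immediately if the commit fails.
; On commit, the instigator's ability system builds a GEDamaged spec with the event's context, which the target's ability system applies to itself.
; It then plays the hit montage and ends when that completes, blends out, is interrupted or cancelled.
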(event `self.K2_ActivateAbilityFromEvent`
  (params (EventData :type "GameplayEventData Structure (by ref)"))
  (set `self.Hit Data` EventData)
  (bind _returnvalue (`self.K2_CommitAbility`))
  (if (not _returnvalue)
    (`self.K2_EndAbility`)))

(event `self.K2_CommitExecute`
  (bind (_eventtag _instigator _target _optionalobject _optionalobject2 _contexthandle) (break `GameplayEventData` (`self.Hit Data`)))
  (`AbilitySystemComponent.BP_ApplyGameplayEffectSpecToSelf` (`AbilitySystemBlueprintLibrary.GetAbilitySystemComponent` _target) (`AbilitySystemComponent.MakeOutgoingSpec` (`AbilitySystemBlueprintLibrary.GetAbilitySystemComponent` _instigator) (`self.GE_Damaged`) 0.0 _contexthandle))
  (`AbilityTask_PlayMontageAndWait.CreatePlayMontageAndWaitProxy` "None" (`self.HitMontage`)
    (:`OnCompleted`
      _)
    (:`OnBlendOut`
      _)
    (:`OnInterrupted`
      _)
    (:`OnCancelled`
      _))
  (`self.K2_EndAbility`))

(event `self.K2_OnEndAbility`
  (params (bWasCancelled :type Boolean)))