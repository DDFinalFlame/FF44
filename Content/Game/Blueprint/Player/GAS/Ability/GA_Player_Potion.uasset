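; Player Gameplay Ability for drinking a healing potion.
; With a weapon equipped it only triggers the unequip ability and ends; otherwise it commits, playing the drink montage from CommitExecute.
; Montage notifies drive the action: begin slows walking and attaches a potion actor to the Item socket, while Potion_Drink end applies the heal effect.
; Ending the ability destroys the potion but does not restore walk speed here.
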(event `self.K2_ActivateAbility`
  (bind _asbase_player (cast `BasePlayer` (`.AvatarActor` (break `GameplayAbilityActorInfo` (`self.GetActorInfo`)))))
  (set `self.Base Player` _asbase_player)
  (bind _returnvalue (`AbilitySystemBlueprintLibrary.GetAbilitySystemComponent` _asbase_player))
  (if (`GameplayTagAssetInterface.HasMatchingGameplayTag` _returnvalue (struct :`TagName` "State.Player.Weapon.Equip"))
    (`AbilitySystemComponent.TryActivateAbilityByClass` _returnvalue "/Game/Game/Blueprint/Player/GAS/Ability/GA_Player_UnEquipWeapon.GA_Player_UnEquipWeapon_C" true)
    (`self.K2_EndAbility`)
    (else
      (`self.K2_CommitAbility`)
      (if (not true)
        (`self.K2_EndAbility`)))))

(event `self.K2_CommitExecute`
  (bind _notifyname (`|PlayMontage` (`Character.Mesh` (`self.Base Player`)) "/Game/Assets/SkeletalMesh/Player/Warrior/Animations/Sequence/Potion/AM_DrinkPotion.AM_DrinkPotion")
    (:`OnCompleted`
      (`self.K2_EndAbility` :!label _label))
    (:`OnBlendOut`
      (goto _label))
    (:`OnInterrupted`
      (goto _label))
    (:`OnNotifyBegin`
      (set `CharacterMovementComponent.MaxWalkSpeed` 100.0 (`Character.CharacterMovement` (`self.Base Player`)))
      (bind _returnvalue (`|SpawnActorFromClass` (`self.Potioin Class`) (`KismetMathLibrary.MakeTransform` (0.0 0.0 0.0)) "Undefined" "MultiplyWithRoot" null null))
      (bind _output_get (set `self.Potion` _returnvalue))
      (`Actor.K2_AttachToComponent` _output_get (`Character.Mesh` (`self.Base Player`)) "Item" "KeepRelative" "KeepRelative" "KeepRelative" true))
    (:`OnNotifyEnd`
      (if (== _notifyname "Potion_Drink")
        (bind _returnvalue_2 (`AbilitySystemBlueprintLibrary.MakeSpecHandleByClass` (`self.HealEffect`) (`self.Base Player`)))
        (`self.K2_ApplyGameplayEffectSpecToOwner` _returnvalue_2)))))

(event `self.K2_OnEndAbility`
  (params (bWasCancelled :type Boolean))
  (bind _potion (`self.Potion`)
    (:`then`
      (`Actor.K2_DetachFromActor` _potion "KeepRelative" "KeepRelative" "KeepRelative")
      (`Actor.K2_DestroyActor` _potion))
    (:`else`)))