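; Player Gameplay Ability that equips a weapon by playing a two-handed equip montage on the BasePlayer mesh after a successful commit.
; A montage notify begin lowers walk speed, and the end of the "Equiping" notify calls EquipWeapon on the player.
; The ability ends when the montage completes, blends out or is interrupted, then adds and removes configured loose gameplay tags without replication.
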(event `self.K2_ActivateAbility`
  (bind _asbase_player (cast `BasePlayer` (`.AvatarActor` (break `GameplayAbilityActorInfo` (`self.GetActorInfo`)))))
  (set `self.Base Player` _asbase_player)
  (bind _returnvalue (`self.K2_CommitAbility`))
  (if (not _returnvalue)
    (`self.K2_EndAbility`)))

(event `self.K2_CommitExecute`
  (bind _notifyname (`|PlayMontage` (`Character.Mesh` (`self.Base Player`)) "/Game/Assets/SkeletalMesh/Player/Warrior/Animations/Sequence/Equip/AM_TwoHanded_Equip.AM_TwoHanded_Equip")
    (:`OnCompleted`
      (`self.K2_EndAbility` :!label _label))
    (:`OnBlendOut`
      (goto _label))
    (:`OnInterrupted`
      (goto _label))
    (:`OnNotifyBegin`
      (set `CharacterMovementComponent.MaxWalkSpeed` 100.0 (`Character.CharacterMovement` (`self.Base Player`))))
    (:`OnNotifyEnd`
      (if (== _notifyname "Equiping")
        (`BasePlayer.EquipWeapon` (`self.Base Player`))))))

(event `self.K2_OnEndAbility`
  (params (bWasCancelled :type Boolean))
  (`self.Base Player`
    (:`then`
      (`AbilitySystemBlueprintLibrary.AddLooseGameplayTags` (`self.Base Player`) (`self.Add Tags`))
      (`AbilitySystemBlueprintLibrary.RemoveLooseGameplayTags` (`self.Base Player`) (`self.Remove Tags`)))
    (:`else`)))