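; Gameplay Ability for the player's first attack, which plays an attack montage on the owning BasePlayer.
; After committing, it caches the player's BaseWeapon and ends when the montage completes or is interrupted.
; The Enable_Attack montage notify window switches the weapon's collision to query-only, then back off.
; OnEndAbility also disables that collision if the weapon is valid, so it does not stay active after the ability ends.
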(event `self.K2_ActivateAbility`
  (bind _returnvalue (`self.K2_CommitAbility`))
  (if _returnvalue
    (`|ExecutionSequence`
      (:`then_0`
        (bind _asbase_player (cast `BasePlayer` (`.OwnerActor` (break `GameplayAbilityActorInfo` (`self.GetActorInfo`)))))
        (bind _asbase_weapon (cast `BaseWeapon` (`BasePlayer.Weapon` _asbase_player)))
        (set `self.Weapon` _asbase_weapon))
      (:`then_1`
        (bind _notifyname (`|PlayMontage` (`Character.Mesh` _asbase_player) (`self.AttackMontage`))
          (:`OnCompleted`
            (`self.K2_EndAbility` :!label _label))
          (:`OnInterrupted`
            (goto _label))
          (:`OnNotifyBegin`
            (bind _returnvalue_2 (== _notifyname "Enable_Attack"))
            (if _returnvalue_2
              (`PrimitiveComponent.SetCollisionEnabled` (`BaseWeapon.WeaponCollision` (`self.Weapon`)) "QueryOnly")))
          (:`OnNotifyEnd`
            (if _returnvalue_2
              (`PrimitiveComponent.SetCollisionEnabled` (`BaseWeapon.WeaponCollision` (`self.Weapon`)) "NoCollision"))))))
    (else
      (`self.K2_EndAbility`))))

(event `self.K2_OnEndAbility`
  (params (bWasCancelled :type Boolean))
  (bind _weapon (`self.Weapon`)
    (:`then`
      (`PrimitiveComponent.SetCollisionEnabled` (`BaseWeapon.WeaponCollision` _weapon) "NoCollision"))
    (:`else`)))