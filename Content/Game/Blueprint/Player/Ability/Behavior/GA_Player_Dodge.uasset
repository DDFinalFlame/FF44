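; Player dodge gameplay ability that plays a directional dodge montage on the owning BasePlayer's mesh.
; After committing, it casts the owner and maps the current input direction to a front, back, left or right montage, with two directions sharing the front one.
; The ability ends when the montage completes or is interrupted, or the cast fails, and resets the selection to front on end.
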(event `self.K2_ActivateAbility`
  (bind _returnvalue (`self.K2_CommitAbility`))
  (if _returnvalue
    (bind _asbase_player (cast `BasePlayer` (`.OwnerActor` (break `GameplayAbilityActorInfo` (`self.GetActorInfo`))))
      (:`then`
        (bind _output_get (set `self.BasePlayer` _asbase_player))
        (`|ExecutionSequence`
          (:`then_0`
            (switch `int` (`BasePlayer.GetCurrentInputDirection` _output_get)
              (:`0`
                (set `self.Current_Dodge` (`self.Dodge_Front`) :!label _label))
              (:`1`
                (goto _label))
              (:`2`
                (set `self.Current_Dodge` (`self.Dodge_Back`)))
              (:`3`
                (set `self.Current_Dodge` (`self.Dodge_Left`)))
              (:`4`
                (set `self.Current_Dodge` (`self.Dodge_Right`)))))
          (:`then_1`
            (`|PlayMontage` (`Character.Mesh` (`self.BasePlayer`)) (`self.Current_Dodge`) 1.0 0.0 "None"
              (:`OnCompleted`
                _)
              (:`OnInterrupted`
                _))
            (`self.K2_EndAbility`))))
      (:`CastFailed`
        (`self.K2_EndAbility`)))))

(event `self.K2_OnEndAbility`
  (params (bWasCancelled :type Boolean))
  (set `self.Current_Dodge` (`self.Dodge_Front`)))