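; Gameplay Ability that equips the player's weapon.
; On activation it commits the ability, casts the owner actor to BasePlayer, calls EquipWeapon and ends immediately.
; When the ability ends, it adds and removes configured loose gameplay tags on the owner without replication.
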(event `self.K2_ActivateAbility`
  (bind _returnvalue (`self.K2_CommitAbility`))
  (if _returnvalue
    (bind _asbase_player (cast `BasePlayer` (`.OwnerActor` (break `GameplayAbilityActorInfo` (`self.GetActorInfo`)))))
    (`BasePlayer.EquipWeapon` _asbase_player)
    (`self.K2_EndAbility`)))

(event `self.K2_OnEndAbility`
  (params (bWasCancelled :type Boolean))
  (bind _owneractor (break `GameplayAbilityActorInfo` (`self.GetActorInfo`)))
  (`AbilitySystemBlueprintLibrary.AddLooseGameplayTags` _owneractor (`self.Add Tags`))
  (`AbilitySystemBlueprintLibrary.RemoveLooseGameplayTags` _owneractor (`self.Remove Tags`)))