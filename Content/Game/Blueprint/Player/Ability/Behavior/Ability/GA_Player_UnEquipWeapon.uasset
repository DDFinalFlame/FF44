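; Gameplay ability that unequips the player's weapon.
; On activation it commits, casts the owner actor to BasePlayer, calls UnEquipWeapon and ends immediately; a failed commit or cast leaves it without an EndAbility call.
; When the ability ends, it adds the AddTags and removes the RemoveTags as non-replicated loose gameplay tags.
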(event `self.K2_ActivateAbility`
  (bind _returnvalue (`self.K2_CommitAbility`))
  (if _returnvalue
    (bind _asbase_player (cast `BasePlayer` (`.OwnerActor` (break `GameplayAbilityActorInfo` (`self.GetActorInfo`)))))
    (`BasePlayer.UnEquipWeapon` _asbase_player)
    (`self.K2_EndAbility`)))

(event `self.K2_OnEndAbility`
  (params (bWasCancelled :type Boolean))
  (`AbilitySystemBlueprintLibrary.AddLooseGameplayTags` null (`self.Add Tags`))
  (`AbilitySystemBlueprintLibrary.RemoveLooseGameplayTags` null (`self.Remove Tags`)))